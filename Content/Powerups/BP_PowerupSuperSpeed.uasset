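; Super speed powerup that temporarily makes the activating actor walk faster.
; On activation it runs the parent logic, stores the target and sets its CharacterMovementComponent max walk speed to one and a half times DefaultSpeed.
; On expiry it sets the stored target back to DefaultSpeed, rather than a captured previous speed, then runs the parent expiry logic even if no movement component is found.
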(event EventOnExpired
  (bind _activate_for_player (Variables|Default|GetActivate%20For%20Player))
  (bind _returnvalue (Actor|GetComponentbyClass _activate_for_player "/Script/Engine.CharacterMovementComponent"))
  (Utilities|IsValid _returnvalue
    (:Is%20Valid
      (Variables|/Script/Engine.CharacterMovementComponent|SetMaxWalkSpeed _returnvalue (Variables|Default|GetDefaultSpeed))
      (|CallParentFunction))
    (:Is%20Not%20Valid
      (|CallParentFunction))))

(event EventOnActivated
  (params (ActivateFor :type Actor%20Object%20Reference))
  (bind _returnvalue (Actor|GetComponentbyClass ActivateFor "/Script/Engine.CharacterMovementComponent"))
  (|CallParentFunction 0)
  (Variables|Default|SetActivate%20For%20Player ActivateFor)
  (Utilities|IsValid _returnvalue
    (:Is%20Valid
      (Variables|/Script/Engine.CharacterMovementComponent|SetMaxWalkSpeed _returnvalue (* (Variables|Default|GetDefaultSpeed) 1.5)))))

(fn ConstructionScript)