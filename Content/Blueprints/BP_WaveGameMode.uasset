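; Wave game mode that spawns enemy bots and awards score for kills.
; SpawnNewBot runs an EQS query for spawn locations, then draws a debug sphere and spawns a weighted-random bot at each result, favoring trackers over rifle or launcher AI.
; An actor-killed handler adds a fixed score to the killer's TPSPlayerState, ignoring player character and explosive barrel victims.
; Wave timing and SpawnNewBot's caller are outside this graph.
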(event Custom|OnQueryFinishedEvent
  (params (QueryInstance :type Env%20Query%20Instance%20Blueprint%20Wrapper%20Object%20Reference) (QueryStatus :type EEnvQueryStatus%20Enum :default "Processing"))
  (switch Utilities|FlowControl|Switch|SwitchonEEnvQueryStatus QueryStatus
    (:Success
      (bind _resultlocations (AI|EQS|GetQueryResultsasLocations QueryInstance))
      (for _array_element _resultlocations
        (Rendering|Debug|DrawDebugSphere _array_element 5e+01 12 "(R=1.000000,G=1.000000,B=0.000000,A=1.000000)" 2.0 2.0)
        (Game|SpawnActorfromClass (select (<= (Math|Random|RandomFloatinRange 0.0 1e+02) 35.0) (select (Math|Random|RandomBool) "/Game/AdvancedAI/BP_AdvancedAI_Launcher.BP_AdvancedAI_Launcher_C" "/Game/AdvancedAI/BP_AdvancedAI_Rifle.BP_AdvancedAI_Rifle_C") "/Game/TrackerBot/BP_TrackerBot.BP_TrackerBot_C") (Math|Transform|MakeTransform _array_element) "AdjustIfPossibleButDontSpawnIfColliding" 0 0)))))

(event Custom|OnActorKilledEvent
  (params (VictimActor :type Actor%20Object%20Reference) (KillerActor :type Actor%20Object%20Reference) (KillerController :type Controller%20Object%20Reference))
  (bind _returnvalue (Pawn|GetControlledPawn KillerController))
  (Utilities|Casting|CastToBP_Character VictimActor
    (:CastFailed
      (Utilities|Casting|CastToBP_ExplosiveBarrel VictimActor
        (:CastFailed
          (Utilities|IsValid KillerController
            (:Is%20Valid
              (Utilities|IsValid _returnvalue
                (:Is%20Valid
                  (bind _astpsplayer_state (Utilities|Casting|CastToTPSPlayerState (Variables|/Script/Engine.Pawn|GetPlayerState _returnvalue)))
                  (Class|TPSPlayerState|AddScore _astpsplayer_state 2e+01))))))))))

(event EventBeginPlay
  (EventDispatchers|AssignOnActorKilled (delegate Custom|OnActorKilledEvent)))

(event EventSpawnNewBot
  (bind _returnvalue (AI|EQS|RunEQSQuery "/Game/Blueprints/EQS_FindSpawnLocation.EQS_FindSpawnLocation" self "RandomBest25Pct"))
  (EventDispatchers|AssignOnQueryFinishedEvent _returnvalue (delegate Custom|OnQueryFinishedEvent)))

(fn ConstructionScript)