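; BP_TargetDummy is a target dummy actor that visualizes incoming damage and never stays dead.
; Point damage draws a short-lived debug sphere and the damage value at the hit location.
; Radial damage draws the same markers at a fixed height above the actor's location.
; When its TPSHealth component reports health at or below zero, it resets that health.
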(event OnHealthChanged(TPSHealth)
  (params (InHealthComp :type TPS%20Health%20Component%20Object%20Reference) (CurrentHealth :type Float%20%28single-precision%29) (HealthDelta :type Float%20%28single-precision%29) (DamageType :type Damage%20Type%20Object%20Reference) (InstigatedBy :type Controller%20Object%20Reference) (DamageCauser :type Actor%20Object%20Reference))
  (if (<= CurrentHealth 0.0)
    (Class|TPSHealthComponent|ResetCurrentHeath (Variables|Default|GetTPSHealth))))

(event EventBeginPlay)

(event Collision|EventActorBeginOverlap
  (params (OtherActor :type Actor%20Object%20Reference)))

(event EventTick
  (params (DeltaSeconds :type Float%20%28single-precision%29)))

(event Game|Damage|EventPointDamage
  (params (Damage :type Float%20%28single-precision%29) (DamageType :type Damage%20Type%20Object%20Reference) (HitLocation :type Vector :default "0, 0, 0") (HitNormal :type Vector :default "0, 0, 0") (HitComponent :type Primitive%20Component%20Object%20Reference) (BoneName :type Name :default "None") (ShotFromDirection :type Vector :default "0, 0, 0") (InstigatedBy :type Controller%20Object%20Reference) (DamageCauser :type Actor%20Object%20Reference) (HitInfo :type Hit%20Result%20Structure%20%28by%20ref%29))
  (Rendering|Debug|DrawDebugSphere HitLocation 5.0 12 "(R=1.000000,G=1.000000,B=0.000000,A=1.000000)" 1.0 1.0)
  (Rendering|Debug|DrawDebugString HitLocation (Utilities|String|ToString(Float) Damage) 0 "(R=1.000000,G=1.000000,B=1.000000,A=1.000000)" 1.0))

(event Game|Damage|EventRadialDamage
  (params (DamageReceived :type Float%20%28single-precision%29) (DamageType :type Damage%20Type%20Object%20Reference) (Origin :type Vector :default "0, 0, 0") (HitInfo :type Hit%20Result%20Structure%20%28by%20ref%29) (InstigatedBy :type Controller%20Object%20Reference) (DamageCauser :type Actor%20Object%20Reference))
  (bind _returnvalue (Transformation|GetActorLocation))
  (bind (_x _y _z) (Math|Vector|BreakVector _returnvalue))
  (bind _returnvalue_2 (+ _z 1e+02))
  (bind _returnvalue_3 (Math|Vector|MakeVector _x _y _returnvalue_2))
  (Rendering|Debug|DrawDebugSphere _returnvalue_3 5.0 12 "(R=1.000000,G=1.000000,B=0.000000,A=1.000000)" 1.0 1.0)
  (Rendering|Debug|DrawDebugString _returnvalue_3 (Utilities|String|ToString(Float) DamageReceived) 0 "(R=1.000000,G=1.000000,B=1.000000,A=1.000000)" 1.0))

(fn ConstructionScript)